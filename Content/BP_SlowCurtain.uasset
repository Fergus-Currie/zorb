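; BP_SlowCurtain is a zone that slows the player character and ai_zorber AI through separate overlap boxes.
; While the player overlaps Playerbox, Tick damps the capsule's horizontal physics velocity each frame, independent of delta time, leaving vertical speed intact.
; Aibox overlaps toggle the zorber's own Triggered flag and lower or restore its Topspeed.
; Tick's matching AI damping requires the player trigger plus TriggeredAI, which nothing here sets.
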(event OnComponentEndOverlap(playerbox)
  (params (OverlappedComponent :type Primitive%20Component%20Object%20Reference) (OtherActor :type Actor%20Object%20Reference) (OtherComp :type Primitive%20Component%20Object%20Reference) (OtherBodyIndex :type Integer))
  (if (Variables|Default|GetTriggered)
    (Variables|Default|SetTriggered false)))

(event OnComponentBeginOverlap(playerbox)
  (params (OverlappedComponent :type Primitive%20Component%20Object%20Reference) (OtherActor :type Actor%20Object%20Reference) (OtherComp :type Primitive%20Component%20Object%20Reference) (OtherBodyIndex :type Integer) (bFromSweep :type Boolean) (SweepResult :type Hit%20Result%20Structure%20%28by%20ref%29))
  (bind _asbp_third_person_character (Utilities|Casting|CastToBP_ThirdPersonCharacter OtherActor))
  (bind _output_get (Variables|Default|SetAs%20BP%20Third%20Person%20Character _asbp_third_person_character))
  (if (not (Variables|Default|GetTriggered))
    (Variables|Default|SetTriggered true)))

(event OnComponentBeginOverlap(aibox)
  (params (OverlappedComponent :type Primitive%20Component%20Object%20Reference) (OtherActor :type Actor%20Object%20Reference) (OtherComp :type Primitive%20Component%20Object%20Reference) (OtherBodyIndex :type Integer) (bFromSweep :type Boolean) (SweepResult :type Hit%20Result%20Structure%20%28by%20ref%29))
  (bind _asai_zorber (Utilities|Casting|CastToai_zorber OtherActor))
  (bind _output_get (Variables|Default|SetAs%20Ai%20Zorber _asai_zorber))
  (if (not (Variables|/Game/Characters/AI_zorbers/ai_zorber.ai_zorber_C|GetTriggered _output_get))
    (Variables|/Game/Characters/AI_zorbers/ai_zorber.ai_zorber_C|SetTriggered _output_get true)
    (Variables|/Game/Characters/AI_zorbers/ai_zorber.ai_zorber_C|SetTopspeed _output_get 3e+03)))

(event OnComponentEndOverlap(aibox)
  (params (OverlappedComponent :type Primitive%20Component%20Object%20Reference) (OtherActor :type Actor%20Object%20Reference) (OtherComp :type Primitive%20Component%20Object%20Reference) (OtherBodyIndex :type Integer))
  (bind _asai_zorber (Utilities|Casting|CastToai_zorber OtherActor))
  (if (Variables|/Game/Characters/AI_zorbers/ai_zorber.ai_zorber_C|GetTriggered _asai_zorber)
    (Variables|/Game/Characters/AI_zorbers/ai_zorber.ai_zorber_C|SetTriggered _asai_zorber false)
    (Variables|/Game/Characters/AI_zorbers/ai_zorber.ai_zorber_C|SetTopspeed _asai_zorber 1e+04)))

(event EventTick
  (params (DeltaSeconds :type Float%20%28single-precision%29))
  (if (Variables|Default|GetTriggered)
    (Class|PrimitiveComponent|SetAllPhysicsLinearVelocity (Variables|/Script/Engine.Character|GetCapsuleComponent (stale OnComponentBeginOverlap(playerbox) _output_get)) (* (Transformation|GetVelocity (stale OnComponentBeginOverlap(playerbox) _output_get)) "0.960000,0.960000,1.000000") false)
    (if (Variables|Default|GetTriggered_AI)
      (Class|PrimitiveComponent|SetAllPhysicsLinearVelocity (Variables|/Script/Engine.Character|GetCapsuleComponent (stale OnComponentBeginOverlap(aibox) _output_get)) (* (Transformation|GetVelocity (stale OnComponentBeginOverlap(aibox) _output_get)) "0.960000,0.960000,1.000000") false))))

(fn ConstructionScript)