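; BP_TrackSpline is a track-building actor that lays a repeated mesh along its spline.
; The Construction Script adds one X-forward spline mesh component per whole SplineLengthOfMesh interval, leaving any shorter remainder at the end uncovered.
; Each segment takes local positions and tangents from the spline at its two ends, with tangent size clamped to the segment length.
; It has no runtime logic.
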(event EventBeginPlay)

(event Collision|EventActorBeginOverlap
  (params (OtherActor :type Actor%20Object%20Reference)))

(event EventTick
  (params (DeltaSeconds :type Float%20%28single-precision%29)))

(fn ConstructionScript
  (bind _spline (Variables|Default|GetSpline))
  (bind _output_get (Variables|Default|SetSplineLengthOfMesh (Variables|Default|GetSplineLengthOfMesh)))
  (for _index (range 0 (- (Math|Float|Truncate (/ (Spline|GetSplineLength (Variables|Default|GetSpline)) _output_get)) 1))
    (bind _returnvalue (AddComponent|AddSplineMeshComponent false))
    (SplineMesh|SetForwardAxis _returnvalue "X" true)
    (Components|StaticMesh|SetStaticMesh _returnvalue (Variables|Default|GetMeshOnSpline))
    (SplineMesh|SetStartandEnd _returnvalue (Spline|GetLocationatDistanceAlongSpline _spline (* (Variables|Default|GetSplineLengthOfMesh) (Math|Conversions|ToFloat(Integer) _index)) "Local") (Math|Vector|ClampVectorSize (Spline|GetTangentatDistanceAlongSpline _spline (* (Variables|Default|GetSplineLengthOfMesh) (Math|Conversions|ToFloat(Integer) _index)) "Local") 0.0 (Variables|Default|GetSplineLengthOfMesh)) (Spline|GetLocationatDistanceAlongSpline _spline (* (Variables|Default|GetSplineLengthOfMesh) (Math|Conversions|ToFloat(Integer) (+ _index 1))) "Local") (Math|Vector|ClampVectorSize (Spline|GetTangentatDistanceAlongSpline _spline (* (Variables|Default|GetSplineLengthOfMesh) (Math|Conversions|ToFloat(Integer) (+ _index 1))) "Local") 0.0 (Variables|Default|GetSplineLengthOfMesh)) true :!class /Script/Engine.SplineMeshComponent)))